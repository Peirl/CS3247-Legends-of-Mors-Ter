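; Destructible rock actor that the player breaks by pressing E while in range.
; Any actor overlap sets an in-range flag and enables input from the first player controller; ending overlap clears the flag but leaves input enabled.
; Pressing E while flagged applies radius damage to the DestructibleComponent at the actor's location, then immediately destroys the whole actor.
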(event EventBeginPlay)

(event EventTick
  (params (DeltaSeconds :type Float%20%28single-precision%29)))

(event Collision|EventActorBeginOverlap
  (params (OtherActor :type Actor%20Object%20Reference))
  (Variables|Default|Setinrange true)
  (Input|EnableInput (Game|GetPlayerController 0)))

(event Collision|EventActorEndOverlap
  (params (OtherActor :type Actor%20Object%20Reference))
  (Variables|Default|Setinrange false))

(event Input|KeyboardEvents|E
  (params (Key :type Key%20Structure :default "AnyKey"))
  (:Pressed
    (if (Variables|Default|Getinrange)
      (Class|DestructibleComponent|ApplyRadiusDamage (Variables|Default|GetDestructibleComponent) 1.0 (Transformation|GetActorLocation) 1.0 1.0 false)
      (Actor|DestroyActor))))

(fn ConstructionScript)