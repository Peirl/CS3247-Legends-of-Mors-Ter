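; BP_RuinedCastle is a ruined castle actor that plays falling-brick effects when it spawns.
; On BeginPlay it prints a debug message and calls SpawnBrickFallEffect for each of its four tower components.
; That function spawns the P_BricksFall emitter at a fixed height above the given tower's world location.
; An unconnected variant that offsets the emitter by castle radius and height remains in the function but never runs.
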(event EventBeginPlay
  (Development|PrintString "Spawned Castle")
  (CallFunction|SpawnBrickFallEffect (Variables|Default|GetCastleTower1))
  (CallFunction|SpawnBrickFallEffect (Variables|Default|GetCastleTower2))
  (CallFunction|SpawnBrickFallEffect (Variables|Default|GetCastleTower3))
  (CallFunction|SpawnBrickFallEffect (Variables|Default|GetCastleTower4)))

(fn ConstructionScript)

(fn SpawnBrickFallEffect
  (params (Tower :type Static%20Mesh%20Component%20Object%20Reference))
  (Effects|SpawnEmitteratLocation "/Game/ProjectAssets/Effects/P_BricksFall.P_BricksFall" (+ (Transformation|GetWorldLocation Tower) "0, 0,1000.000000"))
  (return))