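; Breakable ceramic pot that drops gold loot when it takes damage or a DragonCharacter overlaps it.
; Damage and overlap each pass through a DoOnce; damage also sets IsGone to block later overlap breaks.
; SpawnLoot places a gold pickup just along the player's forward vector from the pot, matching the player's rotation.
; DestroyPot calls DestroyBreakable with a ceramic break effect and a broken-pot mesh.
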(event EventTakeDamage
  (params (Damage :type Float%20%28single-precision%29) (damage%20At%20Location :type Vector :default "0, 0, 0"))
  (Utilities|FlowControl|DoOnce false
    (:Completed
      (Variables|Default|SetisGone true)
      (CallFunction|SpawnLoot (Game|Player|GetPlayerPawn 0))
      (CallFunction|DestroyPot))))

(event Collision|EventActorBeginOverlap
  (params (OtherActor :type Actor%20Object%20Reference))
  (if (not (Variables|Default|GetisGone))
    (Utilities|FlowControl|DoOnce false
      (:Completed
        (bind _asdragon_character (Utilities|Casting|CastToDragonCharacter OtherActor))
        (CallFunction|SpawnLoot _asdragon_character)
        (CallFunction|DestroyPot)))))

(event EventTick
  (params (DeltaSeconds :type Float%20%28single-precision%29)))

(fn ConstructionScript
  (|CallParentFunction))

(fn DestroyPot
  (CallFunction|DestroyBreakable "/Game/ProjectAssets/Effects/P_PotBreak_Ceramic_effect.P_PotBreak_Ceramic_effect" (Variables|Default|GetPot) "/Game/InfinityBladeFireLands/Environments/Fire/Env_Fire_deco/StaticMesh/SM_pot3broken.SM_pot3broken"))

(fn SpawnLoot
  (params (Dragon :type Actor%20Object%20Reference))
  (bind _returnvalue (Game|SpawnActorfromClass "/Game/ProjectAssets/Blueprints/Character/BP_Loot_Editted.BP_Loot_Editted_C" (Math|Transform|MakeTransform (+ (Transformation|GetActorLocation) (Transformation|GetActorForwardVector Dragon)) (Transformation|GetActorRotation Dragon)) "Undefined" 0 0))
  (Variables|/Game/ProjectAssets/Blueprints/Character/BP_Loot_Editted.BP_Loot_Editted_C|SetGoldValue _returnvalue 5)
  (return))