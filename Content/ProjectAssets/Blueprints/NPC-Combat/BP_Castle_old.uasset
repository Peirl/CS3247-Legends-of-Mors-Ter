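; Destructible castle that turns hostile to the player dragon at low human fame and fires arrow volleys.
; Tick checks range and a line trace, running a looping timer where five launchers lob ballistic arrows, four with randomized lead.
; Unprovoked hits cut human fame, and fire deals timed damage.
; Death drops gold loot; direct hits also spawn smoke, falling bricks and a ruined castle, while fire deaths just destroy the actor.
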(event Custom|FireDamage
  (CallFunction|ReduceHitpoint 5.0)
  (bind _isdestoryed (CallFunction|IsDestroyed))
  (if _isdestoryed
    (Utilities|FlowControl|DoOnce false
      (:Completed
        (CallFunction|SpawnLoot (Game|Player|GetPlayerPawn 0))
        (Actor|DestroyActor)))))

(event Custom|OnFire
  (bind _returnvalue (Effects|SpawnEmitteratLocation "/Game/StarterContent/Particles/P_Fire.P_Fire" (+ (Transformation|GetActorLocation) "0, 0,800.000000") "0, 0, 0" false))
  (Transformation|SetRelativeScale3D _returnvalue "25.000000,25.000000,25.000000")
  (bind _returnvalue_2 (Utilities|Time|SetTimerbyEvent (delegate Custom|FireDamage) 1.0 true))
  (Utilities|FlowControl|Delay 5.0)
  (Components|DestroyComponent _returnvalue)
  (Class|KismetSystemLibrary|ClearTimerHandle _returnvalue_2))

(event Custom|destroyOnHit
  (params (hitLocation :type Vector))
  (Game|SpawnActorfromClass "/Game/ProjectAssets/Effects/BP_smoke_castle.BP_smoke_castle_C" (Math|Transform|MakeTransform hitLocation "0, 0, 0" "0.500000,0.500000,1.000000") "Undefined" 0 0)
  (Effects|SpawnEmitteratLocation "/Game/ProjectAssets/Effects/P_BricksFall.P_BricksFall" (+ (Transformation|GetActorLocation) (Math|Vector|MakeVector (Variables|Default|GetcastleRadius) (Variables|Default|GetcastleRadius) (+ (Variables|Default|GetCastleHeight) 2e+01))))
  (Utilities|FlowControl|Delay 2.0)
  (Game|SpawnActorfromClass "/Game/ProjectAssets/Blueprints/NPC-Combat/BP_RuinedCastle_old.BP_RuinedCastle_old_C" (Transformation|GetActorTransform) "Undefined" 0 0)
  (Actor|DestroyActor))

(event EventBeginPlay
  (Variables|Default|SetHitPoint 15.0))

(event EventActorBeginOverlap
  (params (OtherActor :type Actor%20Object%20Reference)))

(event EventTakeDamage
  (params (Damage :type Float%20%28single-precision%29) (damage%20At%20Location :type Vector))
  (CallFunction|CheckPlayerAttack)
  (CallFunction|ReduceHitpoint Damage)
  (bind _isdestoryed (CallFunction|IsDestroyed))
  (if _isdestoryed
    (Utilities|FlowControl|DoOnce false
      (:Completed
        (CallFunction|SpawnLoot (Game|Player|GetPlayerPawn 0))
        (CallFunction|DestroyonHit damage%20At%20Location)))))

(event EventTick
  (params (DeltaSeconds :type Float%20%28single-precision%29))
  (bind _isinrange (CallFunction|GetIsinRange))
  (if _isinrange
    (if (Variables|Default|GetisAttack)
      (Variables|Default|Settarget 0)
      (Utilities|FlowControl|DoOnce false :!label _label
        (:Completed
          (bind _returnvalue (Utilities|Time|SetTimerbyFunctionName 0 "ShootAllArrows" 2.0 true)))))
    (elif (Variables|Default|GetisAttack)
      (Class|KismetSystemLibrary|ClearTimerHandle _returnvalue)
      (goto _label Reset))))

(fn ConstructionScript)

(fn SpawnArrow
  (params (EnemyLocation :type Vector) (Arrow%20location :type Vector) (FlyDuration :type Float%20%28single-precision%29))
  (bind _returnvalue (Game|SpawnActorfromClass "/Game/ProjectAssets/Blueprints/NPC-Combat/BP_Arrow.BP_Arrow_C" (Math|Transform|MakeTransform Arrow%20location) "Undefined" 0 0))
  (Variables|/Script/Engine.MovementComponent|SetVelocity (Variables|/Game/ProjectAssets/Blueprints/NPC-Combat/BP_Arrow.BP_Arrow_C|GetProjectileMovement _returnvalue) (+ (/ (- EnemyLocation Arrow%20location) FlyDuration) (* (* (Math|Vector|MakeVector 0.0 0.0 9.8e+02) 0.5) FlyDuration))))

(fn ShootArrow
  (params (launcher :type Scene%20Component%20Object%20Reference) (prediction :type Boolean))
  (bind _returnvalue (Math|Random|RandomFloatinRange 1.0 2.5))
  (bind _target (Variables|Default|Gettarget))
  (bind _returnvalue_2 (Transformation|GetActorLocation _target))
  (LocalVariables|SetFly%20Duration _returnvalue)
  (if prediction
    (LocalVariables|SetEnemy%20Location (+ _returnvalue_2 (* (Transformation|GetVelocity _target) _returnvalue) (* (Math|Random|RandomUnitVector) (Math|Random|RandomFloatinRange 0.0 1e+02))))
    (else
      (LocalVariables|SetEnemy%20Location _returnvalue_2)))
  (CallFunction|SpawnArrow (LocalVariables|GetEnemy%20Location) (Transformation|GetWorldLocation launcher) (LocalVariables|GetFly%20Duration))
  (return))

(fn IsDestroyed
  (return (<= (Variables|Default|GetHitPoint) 0.0)))

(fn ReduceHitpoint
  (params (Damage :type Float%20%28single-precision%29))
  (bind _output_get (Variables|Default|SetHitPoint (- (Variables|Default|GetHitPoint) Damage)))
  (Development|PrintString (Utilities|String|Append "Castle hp: " (Utilities|String|ToString(Float) _output_get) " Damage:" (Utilities|String|ToString(Float) Damage)))
  (return))

(fn ShootAllArrows
  (CallFunction|ShootArrow (Variables|Default|GetLauncherOne) true)
  (CallFunction|ShootArrow (Variables|Default|GetLauncherTwo) true)
  (CallFunction|ShootArrow (Variables|Default|GetLauncherThree) true)
  (CallFunction|ShootArrow (Variables|Default|GetLauncherFour) true)
  (CallFunction|ShootArrow (Variables|Default|GetLauncherFive) false))

(fn GetIsinRange
  (bind _returnvalue (Game|Player|GetPlayerPawn 0))
  (if (< (Transformation|GetDistanceTo _returnvalue) 1.6e+04)
    (bind _outhit (Collision|LineTraceByChannel (Transformation|GetActorLocation _returnvalue) (Transformation|GetActorLocation) "TraceTypeQuery2" false 0 "ForDuration"))
    (bind _asdragon_character (Utilities|Casting|CastToDragonCharacter (.HitActor (Collision|BreakHitResult _outhit)))
      (:then
        (bind _fame (Default|GetHumanFame _asdragon_character))
        (if (<= _fame -50)
          (Variables|Default|SetisAttack true))
        (return true))
      (:CastFailed
        (return false)))
    (else
      (return false))))

(fn SpawnLoot
  (params (Dragon :type Actor%20Object%20Reference))
  (bind _returnvalue (Game|SpawnActorfromClass "/Game/ProjectAssets/Blueprints/Character/BP_Loot.BP_Loot_C" (Math|Transform|MakeTransform (+ (Transformation|GetActorLocation) (* (Transformation|GetActorForwardVector Dragon) -350)) (Transformation|GetActorRotation Dragon) "1.000000,1.000000,1.000000") "Undefined" 0 0))
  (Variables|/Game/ProjectAssets/Blueprints/Character/BP_Loot.BP_Loot_C|SetGoldValue _returnvalue 50)
  (return))

(fn CheckPlayerAttack
  (bind _returnvalue (Game|Player|GetPlayerPawn 0))
  (if (not (Variables|Default|GetisAttack))
    (bind _fame (Class|BPICharacter|GetHumanFame(Message) _returnvalue))
    (Class|BPICharacter|SetHumanFame(Message) _returnvalue (- _fame 50))))