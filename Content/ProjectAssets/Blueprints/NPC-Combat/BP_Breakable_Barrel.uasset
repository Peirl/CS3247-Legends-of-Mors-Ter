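; Breakable wooden barrel that drops gold loot when it takes damage or a DragonCharacter overlaps it.
; Both triggers spawn a BP_Loot with a fixed gold value, offset from the barrel along the dragon's forward vector and matching its rotation.
; The damage path uses the first player pawn for that direction, regardless of the damage source.
; DestroyBarrel then calls DestroyBreakable with the barrel's particle effect and destroyed mesh.
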(event EventTakeDamage
  (params (Damage :type Float%20%28single-precision%29) (damage%20At%20Location :type Vector :default "0, 0, 0"))
  (CallFunction|SpawnLoot (Game|Player|GetPlayerPawn 0))
  (CallFunction|DestroyBarrel))

(event Collision|EventActorBeginOverlap
  (params (OtherActor :type Actor%20Object%20Reference))
  (bind _asdragon_character (Utilities|Casting|CastToDragonCharacter OtherActor))
  (CallFunction|SpawnLoot _asdragon_character)
  (CallFunction|DestroyBarrel))

(event EventTick
  (params (DeltaSeconds :type Float%20%28single-precision%29)))

(fn ConstructionScript
  (|CallParentFunction))

(fn DestroyBarrel
  (CallFunction|DestroyBreakable "/Game/ProjectAssets/Effects/P_Destroy_Barrel_effect.P_Destroy_Barrel_effect" (Variables|Default|GetBarrel) "/Game/InfinityBladeGrassLands/Environments/Misc/Exo_Deco01/StaticMesh/SM_WoodenBarrel_Destroyed.SM_WoodenBarrel_Destroyed"))

(fn SpawnLoot
  (params (dragon :type Actor%20Object%20Reference))
  (bind _returnvalue (Game|SpawnActorfromClass "/Game/ProjectAssets/Blueprints/Character/BP_Loot.BP_Loot_C" (Math|Transform|MakeTransform (+ (Transformation|GetActorLocation) (* (Transformation|GetActorForwardVector dragon) 100)) (Transformation|GetActorRotation dragon)) "Undefined" 0 0))
  (Variables|/Game/ProjectAssets/Blueprints/Character/BP_Loot.BP_Loot_C|SetGoldValue _returnvalue 5)
  (return 0))