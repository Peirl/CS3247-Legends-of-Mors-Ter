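; Destructible enemy castle NPC that attacks the player with a fire beam when in range and IsAttack is set.
; The beam spawns once after a random delay, then Tick eases its endpoint toward the target and line-traces at fixed intervals to deal damage.
; Hits drain hit points, ending in smoke, falling bricks and destruction.
; OnFire adds a temporary fire emitter with timed damage, which can destroy the castle directly.
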(event Custom|FireDamage
  (CallFunction|ReduceHitpoint 5.0)
  (bind _isdestoryed (CallFunction|IsDestroyed))
  (if _isdestoryed
    (Actor|DestroyActor)))

(event Custom|OnFire
  (bind _returnvalue (Effects|SpawnEmitteratLocation "/Game/StarterContent/Particles/P_Fire.P_Fire" (+ (Transformation|GetActorLocation) "0, 0,800.000000") "0, 0, 0" false))
  (Transformation|SetRelativeScale3D _returnvalue "25.000000,25.000000,25.000000")
  (bind _returnvalue_2 (Utilities|Time|SetTimerbyEvent (delegate Custom|FireDamage) 1.0 true))
  (Utilities|FlowControl|Delay 5.0)
  (Components|DestroyComponent _returnvalue)
  (Class|KismetSystemLibrary|ClearTimerHandle _returnvalue_2))

(event Custom|destroyOnHit
  (params (hitLocation :type Vector))
  (Game|SpawnActorfromClass "/Game/ProjectAssets/Effects/BP_smoke_castle.BP_smoke_castle_C" (Math|Transform|MakeTransform hitLocation "0, 0, 0" "0.500000,0.500000,1.000000") "Undefined" 0 0)
  (Effects|SpawnEmitteratLocation "/Game/ProjectAssets/Effects/P_BricksFall.P_BricksFall" (+ (Transformation|GetActorLocation) (Math|Vector|MakeVector (Variables|Default|GetcastleRadius) (Variables|Default|GetcastleRadius) (+ (Variables|Default|GetCastleHeight) 2e+01))))
  (CallFunction|RemoveBeam)
  (Utilities|FlowControl|Delay 2.0)
  (Actor|DestroyActor))

(event EventBeginPlay
  (Variables|Default|SetHitPoint 15.0))

(event Collision|EventActorBeginOverlap
  (params (OtherActor :type Actor%20Object%20Reference)))

(event EventTakeDamage
  (params (Damage :type Float%20%28single-precision%29) (damage%20At%20Location :type Vector))
  (CallFunction|ReduceHitpoint Damage)
  (bind _isdestoryed (CallFunction|IsDestroyed))
  (if _isdestoryed
    (CallFunction|DestroyonHit damage%20At%20Location)))

(event EventTick
  (params (DeltaSeconds :type Float%20%28single-precision%29))
  (bind (_player _withinrange) (|player))
  (Utilities|FlowControl|Sequence
    (:then_0
      (if _withinrange
        (if (Variables|Default|GetisAttack)
          (Variables|Default|Settarget _player)
          (Utilities|FlowControl|DoOnce false
            (:Completed
              (bind (_source _target _delay) (CallFunction|LocateBeam (Variables|Default|GetLauncherOne) false))
              (Variables|Default|SetcurBeamTarget _target)
              (Utilities|FlowControl|Delay _delay)
              (CallFunction|SpawnBeam _target _source)
              (Variables|Default|Setattacking true)))
          (else
            (Variables|Default|Setattacking false :!label _label)
            (Variables|Default|SetattackLoop 0.0)
            (CallFunction|RemoveBeam)))
        (else
          (goto _label))))
    (:then_1
      (if (Variables|Default|Getattacking)
        (Variables|Default|SetattackLoop (+ (Variables|Default|GetattackLoop) DeltaSeconds))
        (if (> (Variables|Default|GetattackLoop) 0.1)
          (Variables|Default|SetattackLoop (- (Variables|Default|GetattackLoop) 0.1))
          (CallFunction|HomingLoc)
          (CallFunction|MoveBeam (Variables|Default|GetcurBeamTarget))
          (bind _outhit (Collision|LineTraceByChannel (Transformation|GetWorldLocation (Variables|Default|GetLauncherOne)) (Variables|Default|GetcurBeamTarget) "TraceTypeQuery1" false 0 "None"))
          (if (== (.HitActor (Collision|BreakHitResult _outhit)) (Variables|Default|Gettarget))
            (Class|BPITakeDamage|TakeDamage(Message) (Variables|Default|Gettarget) 1.0 (.Location (Collision|BreakHitResult _outhit)))))))))

(fn ConstructionScript)

(fn SpawnBeam
  (params (EnemyLocation :type Vector) (source :type Vector))
  (bind _returnvalue (Effects|SpawnEmitteratLocation "/Game/ProjectAssets/Effects/P_Fire_Beam.P_Fire_Beam" source))
  (Variables|Default|Setbeam _returnvalue)
  (Class|ParticleSystemComponent|SetBeamTargetPoint _returnvalue 0 EnemyLocation))

(fn LocateBeam
  (params (launcher :type Scene%20Component%20Object%20Reference) (prediction :type Boolean))
  (bind _returnvalue (Math|Random|RandomFloatinRange 1.0 2.5))
  (bind _target (Variables|Default|Gettarget))
  (bind _returnvalue_2 (Transformation|GetActorLocation _target))
  (LocalVariables|SetFly%20Duration _returnvalue)
  (if prediction
    (LocalVariables|SetEnemy%20Location (+ _returnvalue_2 (* (Transformation|GetVelocity _target) _returnvalue) (* (Math|Random|RandomUnitVector) (Math|Random|RandomFloatinRange 0.0 1e+02))))
    (else
      (LocalVariables|SetEnemy%20Location _returnvalue_2)))
  (return (Transformation|GetWorldLocation launcher) (LocalVariables|GetEnemy%20Location) (LocalVariables|GetFly%20Duration)))

(fn IsDestroyed
  (return (<= (Variables|Default|GetHitPoint) 0.0)))

(fn ReduceHitpoint
  (params (Damage :type Float%20%28single-precision%29))
  (bind _output_get (Variables|Default|SetHitPoint (- (Variables|Default|GetHitPoint) Damage)))
  (Development|PrintString (Utilities|String|Append "Castle hp: " (Utilities|String|ToString(Float) _output_get) " Damage:" (Utilities|String|ToString(Float) Damage)))
  (return))

(fn MoveBeam
  (params (loc :type Vector))
  (Class|ParticleSystemComponent|SetBeamTargetPoint (Variables|Default|Getbeam) 0 loc))

(fn RemoveBeam
  (if (Variables|Default|Getattacking)
    (Components|DestroyComponent (Variables|Default|Getbeam))
    (Variables|Default|Setattacking false)))

(fn HomingLoc
  (Variables|Default|SetcurBeamTarget (+ (/ (- (Transformation|GetActorLocation (Variables|Default|Gettarget)) (Variables|Default|GetcurBeamTarget)) 1e+01) (Variables|Default|GetcurBeamTarget))))