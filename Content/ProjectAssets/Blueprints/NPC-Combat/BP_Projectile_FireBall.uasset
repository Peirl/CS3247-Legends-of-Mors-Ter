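; BP_Projectile_FireBall is a fireball projectile for NPC combat that damages what it overlaps.
; An overlap on its collision component sends a damage message with the hit location to the other actor, then spawns a fire emitter at the projectile and destroys it.
; A blocking hit only plays the emitter and destroys the actor; the physics impulse branch is left unconnected.
; A setScale event resizes the fireball.
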(event OnComponentBeginOverlap(CollisionComponent)
  (params (OtherActor :type Actor%20Object%20Reference) (OtherComp :type Primitive%20Component%20Object%20Reference) (OtherBodyIndex :type Integer) (bFromSweep :type Boolean) (SweepResult :type Hit%20Result%20Structure%20%28by%20ref%29))
  (Class|BPITakeDamage|TakeDamage(Message) OtherActor (Variables|Default|GetDamage) (.Location (Collision|BreakHitResult SweepResult)))
  ;[1 1 1] Spawn death emitter at hit
  (Effects|SpawnEmitteratLocation "/Game/InfinityBladeEffects/Effects/FX_Mobile/Fire/combat/P_FireBall_Strong_MuzzFlash_01.P_FireBall_Strong_MuzzFlash_01" (Transformation|GetActorLocation))
  (Actor|DestroyActor) ; Then destroy this projectile
)

(event Custom|setScale
  (params (scale :type Float%20%28single-precision%29))
  ;[1 1 1] Set the scale of the fireball
  (bind _output_get (Variables|Default|SetScale scale))
  (Transformation|SetActorRelativeScale3D (Math|Vector|MakeVector _output_get _output_get _output_get)))

(event Collision|EventHit
  (params (MyComp :type Primitive%20Component%20Object%20Reference) (Other :type Actor%20Object%20Reference) (OtherComp :type Primitive%20Component%20Object%20Reference) (bSelfMoved :type Boolean) (HitLocation :type Vector :default "0, 0, 0") (HitNormal :type Vector :default "0, 0, 0") (NormalImpulse :type Vector :default "0, 0, 0") (Hit :type Hit%20Result%20Structure%20%28by%20ref%29))
  ;[1 1 1] Spawn death emitter at hit
  (Effects|SpawnEmitteratLocation "/Game/InfinityBladeEffects/Effects/FX_Mobile/Fire/combat/P_FireBall_Strong_MuzzFlash_01.P_FireBall_Strong_MuzzFlash_01" (Transformation|GetActorLocation))
  (Actor|DestroyActor) ; Then destroy this projectile
)

(fn ConstructionScript)