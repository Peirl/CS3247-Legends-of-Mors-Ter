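; Quest manager actor that runs quest trees from a Quests DataTable, with quest state stored in the game mode.
; Starting a tree finds sub-quests by "Tree$" name prefix, activating or queueing each by its prerequisites.
; Activation spawns a handler actor; completion counts repeats, messages the handler and promotes eligible pending quests.
; Semicolon-delimited instruction strings are parsed but their switches are empty; R/E/T print quest lists for debugging.
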(event EventBeginPlay
  (bind _aslegend_of_mors_ter_game_mode (Utilities|Casting|CastToLegendOfMorsTerGameMode (Game|GetGameMode)))
  (Variables|Default|SetGameMode _aslegend_of_mors_ter_game_mode)
  (Input|EnableInput (Game|GetPlayerController 0)))

(event Input|KeyboardEvents|R
  (params (Key :type Key%20Structure :default "AnyKey"))
  ;[1 1 1] Debug
  (:Pressed
    (Development|PrintString "Pending quests:")
    (Default|PrintAllPendingQuests (Variables|Default|GetGameMode))))

(event Input|KeyboardEvents|E
  (params (Key :type Key%20Structure :default "AnyKey"))
  ;[1 1 1] Debug
  (:Pressed
    (Development|PrintString "Active quests:")
    (Default|PrintAllActiveQuests (Variables|Default|GetGameMode))))

(event Input|KeyboardEvents|T
  (params (Key :type Key%20Structure :default "AnyKey"))
  ;[1 1 1] Debug
  (:Pressed
    (Development|PrintString "Completed quests:")
    (Default|PrintAllCompletedQuests (Variables|Default|GetGameMode))))

(fn ConstructionScript)

(fn StartQuestTree
  (params (QuestName :type Name))
  (bind _output_get (LocalVariables|SetName QuestName))
  (bind _issuccess (Default|ActivateQuestTree (Variables|Default|GetGameMode) _output_get))
  (if _issuccess
    (bind _outrownames (DataTable|GetDataTableRowNames "/Game/ProjectAssets/Blueprints/Quest/Quests.Quests"))
    (bind _subquests (|GetAllSubQuests _outrownames (LocalVariables|GetName)))
    (|ActivateOrPendingSubQuests _subquests
      (:Completed
        (return true)))
    (else
      (return false))))

(fn CheckRequirements
  (params (RequiredQuests :type Array%20of%20Names))
  (LocalVariables|Setvalid true)
  (for _array_element RequiredQuests
    (bind _completed (Default|IsQuestCompleted (Variables|Default|GetGameMode) _array_element))
    (LocalVariables|Setvalid (and _completed (LocalVariables|Getvalid))))
  (return (LocalVariables|Getvalid)))

(fn ParseIntoNameArray
  (params (Names :type String))
  (for _array_element (Utilities|String|ParseIntoArray Names ";")
    (Utilities|Array|Add (LocalVariables|Gettemp) (Utilities|String|StringToName _array_element)))
  (return (LocalVariables|Gettemp)))

(fn BelongstoTree
  (params (Child :type Name) (Parent :type Name))
  (return (Utilities|String|StartsWith (Utilities|String|ToString(Name) Child) (Utilities|String|Append (Utilities|String|ToString(Name) Parent) "$") "CaseSensitive")))

(fn ParseInstruction
  (params (Instructions%20String :type String))
  (bind _returnvalue (Utilities|String|ParseIntoArray Instructions%20String " "))
  (Utilities|Array|RemoveIndex _returnvalue)
  (return (Utilities|String|MakeLiteralString (Utilities|Array|Get(acopy) _returnvalue)) _returnvalue))

(fn ParseInstructions
  (params (Intructions%20String :type String))
  (return (Utilities|String|ParseIntoArray Intructions%20String ";")))

(fn ExecuteonCompletedInstructions
  (params (Instructions%20String :type String))
  (bind _instructions (CallFunction|ParseInstructions Instructions%20String))
  (for _array_element _instructions
    (bind _identifier (CallFunction|ParseInstruction _array_element))
    (switch string _identifier)))

(fn ExecuteonActiveInstructions
  (params (Instructions%20String :type String))
  (bind _instructions (CallFunction|ParseInstructions Instructions%20String))
  (for _array_element _instructions
    (bind _identifier (CallFunction|ParseInstruction _array_element))
    (switch string _identifier)))

(fn HandleQuestCompletion
  (params (Quest%20Name :type Name))
  (bind _output_get (LocalVariables|SetName Quest%20Name))
  (bind _returnvalue (Utilities|GetDataTableRow "/Game/ProjectAssets/Blueprints/Quest/Quests.Quests" _output_get)
    (:then
      (switch Utilities|FlowControl|Switch|SwitchonEQuestFlag (.QuestFlag (Utilities|Struct|BreakQuestStruct _returnvalue))
        (:NewEnumerator2
          (|CompleteQuestHandler (.OnQuestCompletedInstructions (Utilities|Struct|BreakQuestStruct _returnvalue)) :!label _label
            (:Success
              (|PromotePendingQuest))))
        (:NewEnumerator0
          (bind _count (Default|IncrementRepeatingQuestCount (Variables|Default|GetGameMode) (LocalVariables|GetName)))
          (if (>= _count (.RepeatAmount (Utilities|Struct|BreakQuestStruct _returnvalue)))
            (goto _label)
            (else
              (bind _questhandler (CallFunction|GetQuestHandler (LocalVariables|GetName)))
              (if (Utilities|IsValid _questhandler)
                (if (== _count (- (.RepeatAmount (Utilities|Struct|BreakQuestStruct _returnvalue)) 1))
                  (Class|BPIQuest|OnFinalCompletion(Message) _questhandler))
                (Default|Update _questhandler)))))))))

(fn HandleQuestActivation
  (params (QuestName :type Name))
  (bind _returnvalue (Utilities|GetDataTableRow "/Game/ProjectAssets/Blueprints/Quest/Quests.Quests" QuestName)
    (:then
      (bind _returnvalue_2 (Game|SpawnActorfromClass (.QuestActorClass (Utilities|Struct|BreakQuestStruct _returnvalue)) (.SpawnTransform (Utilities|Struct|BreakQuestBPInfoStruct (.QuestActorClassInfo (Utilities|Struct|BreakQuestStruct _returnvalue)))) "Undefined" 0 QuestName self _returnvalue))
      (Class|BPIQuest|Start(Message) _returnvalue_2))))

(fn MakeFullQuestName
  (params (QuestTree :type Name) (QuestName :type Name))
  (return (Utilities|String|StringToName (Utilities|String|Append (Utilities|String|ToString(Name) QuestTree) "$" (Utilities|String|ToString(Name) QuestName)))))

(fn GetQuestHandler
  (params (Name :type Name))
  (bind _returnvalue (Utilities|GetDataTableRow "/Game/ProjectAssets/Blueprints/Quest/Quests.Quests" Name)
    (:then
      (bind _outactors (Actor|GetAllActorsOfClass (.QuestActorClass (Utilities|Struct|BreakQuestStruct _returnvalue))))
      (return (Utilities|Array|Get(acopy) _outactors)))
    (:RowNotFound
      (return 0))))

(fn IsonFinalCompletion
  (params (QuestName :type Name))
  (bind _output_get (LocalVariables|SetName QuestName))
  (bind _true (Default|IsQuestActive (Variables|Default|GetGameMode) _output_get))
  (if _true
    (bind _returnvalue (Utilities|GetDataTableRow "/Game/ProjectAssets/Blueprints/Quest/Quests.Quests" (LocalVariables|GetName))
      (:then
        (if (Utilities|Enum|Equal(Enum) (.QuestFlag (Utilities|Struct|BreakQuestStruct _returnvalue)) "NewEnumerator0")
          (bind _count (Default|GetQuestCount (Variables|Default|GetGameMode) (LocalVariables|GetName)))
          (return (== _count (- (.RepeatAmount (Utilities|Struct|BreakQuestStruct _returnvalue)) 1)))
          (else
            (return true)))))
    (else
      (return false))))