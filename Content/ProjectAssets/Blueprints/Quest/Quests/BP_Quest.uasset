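; BP_Quest is a quest object that exposes its QuestStruct data through getter functions.
; Getters return display text, rewards summary, type, flag, repeat amount, active and completed instructions, and quest actor class info.
; The quest tree name is the part of QuestName left of "$".
; The semicolon-separated required quests string is parsed into names prefixed with that tree name, so prerequisites resolve within the same tree.
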(event EventBeginPlay)

(fn ConstructionScript)

(fn GetQuestTitle
  (return (.QuestTitle (Utilities|Struct|BreakQuestStruct (Variables|Default|GetQuestStruct)))))

(fn GetQuestDescription
  (return (.QuestDescription (Utilities|Struct|BreakQuestStruct (Variables|Default|GetQuestStruct)))))

(fn GetRewardsSummary
  (return (.RewardsSummary (Utilities|Struct|BreakQuestStruct (Variables|Default|GetQuestStruct)))))

(fn GetRequiredQuestsString
  (return (.RequiredQuests (Utilities|Struct|BreakQuestStruct (Variables|Default|GetQuestStruct)))))

(fn GetRequiredQuestsParsed
  (bind _questtreename (CallFunction|GetQuestTreeName))
  (for (_array_element _array_index) (Utilities|String|ParseIntoArray (.RequiredQuests (Utilities|Struct|BreakQuestStruct (Variables|Default|GetQuestStruct))) ";")
    (Utilities|Array|SetArrayElem (LocalVariables|GetParsed) _array_index (Utilities|String|StringToName (Utilities|String|Append (Utilities|String|ToString(Name) _questtreename) "$" _array_element))))
  (return (LocalVariables|GetParsed)))

(fn GetQuestType
  (return (.QuestType (Utilities|Struct|BreakQuestStruct (Variables|Default|GetQuestStruct)))))

(fn GetQuestFlag
  (return (.QuestFlag (Utilities|Struct|BreakQuestStruct (Variables|Default|GetQuestStruct)))))

(fn GetRepeatAmount
  (return (.RepeatAmount (Utilities|Struct|BreakQuestStruct (Variables|Default|GetQuestStruct)))))

(fn GetonQuestActiveInstructions
  (return (.OnQuestActiveInstructions (Utilities|Struct|BreakQuestStruct (Variables|Default|GetQuestStruct)))))

(fn GetonQuestCompletedInstructions
  (return (.OnQuestCompletedInstructions (Utilities|Struct|BreakQuestStruct (Variables|Default|GetQuestStruct)))))

(fn GetQuestActorClass
  (return (.QuestActorClass (Utilities|Struct|BreakQuestStruct (Variables|Default|GetQuestStruct)))))

(fn GetQuestActorClassInfo
  (return (.QuestActorClassInfo (Utilities|Struct|BreakQuestStruct (Variables|Default|GetQuestStruct)))))

(fn GetQuestTreeName
  (return (Utilities|String|StringToName (.LeftS (Utilities|String|Split (Utilities|String|ToString(Name) (Variables|Default|GetQuestName)) "$")))))