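; Story menu actor that shows dialogue text and two selectable child-actor options for the game's branching narrative.
; On BeginPlay it finds LegendOfMorsTerGameMode and hands itself and an index to each option.
; SetText routes strings to an option label or to the dialogue, where nested newline splits fill six text lines.
; Selections from options are forwarded to the game mode's PlayerSelectStory, and CloseMenu destroys the actor.
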(event EventBeginPlay
  ;[1 1 1] BeginPlay
  (bind _outactors (Actor|GetAllActorsOfClass "/Game/ProjectAssets/Maps/LegendOfMorsTerGameMode.LegendOfMorsTerGameMode_C"))
  (Variables|Default|SetgameMode (Utilities|Array|Get(acopy) _outactors))
  (CallFunction|InitSelf)
  (Class|BPIOption|SetSelect(Message) (Variables|/Script/Engine.ChildActorComponent|GetChildActor (Variables|Default|GetOption1)))
  (Class|BPIOption|SetSelect(Message) (Variables|/Script/Engine.ChildActorComponent|GetChildActor (Variables|Default|GetOption2)) 1))

(event EventSelectedOption
  (params (selection :type Integer))
  ;[1 1 1] call back from option, call game mode
  (Default|PlayerSelectStory (Variables|Default|GetgameMode) selection self))

(event EventSetId
  (params (iD :type Name))
  ;[1 1 1] interface setId
  (Variables|Default|Setid iD))

(event EventCloseMenu
  ;[1 1 1] interface closeMenu
  (Actor|DestroyActor))

(event EventSetText
  (params (String :type String) (Option :type Integer))
  (bind _returnvalue (Utilities|Text|ToText(String) String))
  ;[1 1 1] Interface setText
  (switch int Option
    (:Default
      (CallFunction|ClearDialogue :!label _label)
      (CallFunction|SetTextSelf String))
    (:0
      (goto _label))
    (:1
      (Class|BPIOption|SetText(Message) (Variables|/Script/Engine.ChildActorComponent|GetChildActor (Variables|Default|GetOption1)) _returnvalue))
    (:2
      (Class|BPIOption|SetText(Message) (Variables|/Script/Engine.ChildActorComponent|GetChildActor (Variables|Default|GetOption2)) _returnvalue))))

(fn ConstructionScript)

(fn SetTextSelf
  (params (String :type String))
  (bind (_lefts _rights _returnvalue) (Utilities|String|Split String "\\n"))
  (bind (_lefts_2 _rights_2 _returnvalue_2) (Utilities|String|Split _rights "\\n"))
  (bind (_lefts_3 _rights_3 _returnvalue_3) (Utilities|String|Split _rights_2 "\\n"))
  (bind (_lefts_4 _rights_4 _returnvalue_4) (Utilities|String|Split _rights_3 "\\n"))
  (bind (_lefts_5 _rights_5 _returnvalue_5) (Utilities|String|Split _rights_4 "\\n"))
  (if _returnvalue
    (Rendering|Components|TextRender|SetText (Variables|Default|GetText1) (Utilities|Text|ToText(String) _lefts))
    (if _returnvalue_2
      (Rendering|Components|TextRender|SetText (Variables|Default|GetText2) (Utilities|Text|ToText(String) _lefts_2))
      (if _returnvalue_3
        (Rendering|Components|TextRender|SetText (Variables|Default|GetText3) (Utilities|Text|ToText(String) _lefts_3))
        (if _returnvalue_4
          (Rendering|Components|TextRender|SetText (Variables|Default|GetText4) (Utilities|Text|ToText(String) _lefts_4))
          (if _returnvalue_5
            (Rendering|Components|TextRender|SetText (Variables|Default|GetText5) (Utilities|Text|ToText(String) _lefts_5))
            (Rendering|Components|TextRender|SetText (Variables|Default|GetText6) (Utilities|Text|ToText(String) _rights_5))
            (else
              (Rendering|Components|TextRender|SetText (Variables|Default|GetText5) (Utilities|Text|ToText(String) _rights_4))))
          (else
            (Rendering|Components|TextRender|SetText (Variables|Default|GetText4) (Utilities|Text|ToText(String) _rights_3))))
        (else
          (Rendering|Components|TextRender|SetText (Variables|Default|GetText3) (Utilities|Text|ToText(String) _rights_2))))
      (else
        (Rendering|Components|TextRender|SetText (Variables|Default|GetText2) (Utilities|Text|ToText(String) _rights))))
    (else
      (Rendering|Components|TextRender|SetText (Variables|Default|GetText1) (Utilities|Text|ToText(String) String))))
  (return))

(fn InitSelf
  (bind _self self)
  (Class|BPIOption|SetMenu(Message) (Variables|/Script/Engine.ChildActorComponent|GetChildActor (Variables|Default|GetOption1)) _self)
  (Class|BPIOption|SetMenu(Message) (Variables|/Script/Engine.ChildActorComponent|GetChildActor (Variables|Default|GetOption2)) _self)
  (return))

(fn ClearDialogue
  (bind _returnvalue (Utilities|String|MakeLiteralString))
  (bind _returnvalue_2 (Utilities|Text|ToText(String) _returnvalue))
  (Rendering|Components|TextRender|SetText (Variables|Default|GetText1) _returnvalue_2)
  (Rendering|Components|TextRender|SetText (Variables|Default|GetText2) _returnvalue_2)
  (Rendering|Components|TextRender|SetText (Variables|Default|GetText3) _returnvalue_2)
  (Rendering|Components|TextRender|SetText (Variables|Default|GetText4) _returnvalue_2)
  (Rendering|Components|TextRender|SetText (Variables|Default|GetText5) _returnvalue_2)
  (Rendering|Components|TextRender|SetText (Variables|Default|GetText6) _returnvalue_2)
  (return))