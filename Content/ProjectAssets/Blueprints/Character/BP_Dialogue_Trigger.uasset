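; BP_Dialogue_Trigger is a trigger actor that shows a named dialogue when the player pawn overlaps it.
; It looks up DialogueName in the LegendOfMorsTerGameMode dialogue array and checks the matching PlayDialogueArray flag.
; If set, it spawns a BP_Dialogue_Renderer in front of the player with that name.
; Ending any overlap sends CloseMenuMessage to the stored renderer if it is valid.
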(event Collision|EventActorEndOverlap
  (params (OtherActor :type Actor%20Object%20Reference))
  (if (Utilities|IsValid (Variables|Default|Getrenderer))
    (Class|BPIMenu|CloseMenu(Message) (Variables|Default|Getrenderer))))

(event EventBeginPlay)

(event Collision|EventActorBeginOverlap
  (params (OtherActor :type Actor%20Object%20Reference))
  (bind _returnvalue (Game|Player|GetPlayerPawn 0))
  (bind _dialoguename (Variables|Default|GetdialogueName))
  (if (== OtherActor _returnvalue)
    (bind _outactors (Actor|GetAllActorsOfClass "/Game/ProjectAssets/Maps/LegendOfMorsTerGameMode.LegendOfMorsTerGameMode_C"))
    (if (Utilities|Array|Get(acopy) (Variables|/Game/ProjectAssets/Maps/LegendOfMorsTerGameMode.LegendOfMorsTerGameMode_C|GetplayDialogueArray (Utilities|Array|Get(acopy) _outactors)) (Utilities|Array|FindItem (Variables|/Game/ProjectAssets/Maps/LegendOfMorsTerGameMode.LegendOfMorsTerGameMode_C|GetdialogueArray (Utilities|Array|Get(acopy) _outactors)) (Variables|Default|GetdialogueName)))
      (Development|PrintString (Utilities|String|ToString(Name) _dialoguename))
      (bind _returnvalue_2 (Game|SpawnActorfromClass "/Game/ProjectAssets/Blueprints/Character/BP_Dialogue_Renderer.BP_Dialogue_Renderer_C" (Math|Transform|MakeTransform (+ (Transformation|GetActorLocation _returnvalue) (* (Transformation|GetActorForwardVector _returnvalue) 5e+02)) (Transformation|GetActorRotation _returnvalue)) "Undefined" 0 _dialoguename 0))
      (Variables|Default|Setrenderer _returnvalue_2))))

(fn ConstructionScript)