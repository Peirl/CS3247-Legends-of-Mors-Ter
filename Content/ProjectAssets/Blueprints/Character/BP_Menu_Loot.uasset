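; BP_Menu_Loot is an in-world loot menu actor showing a "Loot?" prompt with "Next" and "Close" options.
; On BeginPlay it finds the LegendOfMorsTerGameMode, registers itself with two child-actor options and sets their labels through interface-style messages.
; A selection callback forwards an Id-based string and the menu to the game mode's PlayerSelectLoot.
; Interface events also update text by index, reset the Id and destroy the actor on close.
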(event EventBeginPlay
  ;[1 1 1] BeginPlay
  (bind _outactors (Actor|GetAllActorsOfClass "/Game/ProjectAssets/Maps/LegendOfMorsTerGameMode.LegendOfMorsTerGameMode_C"))
  (Variables|Default|SetgameMode (Utilities|Array|Get(acopy) _outactors))
  (CallFunction|InitSelf)
  (CallFunction|SetText "Loot?")
  (CallFunction|SetText "Next" 1)
  (CallFunction|SetText "Close" 2)
  (Class|BPIOption|SetSelect(Message) (Variables|/Script/Engine.ChildActorComponent|GetChildActor (Variables|Default|GetOption1)))
  (Class|BPIOption|SetSelect(Message) (Variables|/Script/Engine.ChildActorComponent|GetChildActor (Variables|Default|GetOption2))))

(event EventSelectedOption
  (params (selection :type Integer))
  ;[1 1 1] call back from option, call game mode
  (Default|PlayerSelectLoot (Variables|Default|GetgameMode) (Utilities|String|Append (Variables|Default|Getid) ".") self))

(event EventSetId
  (params (iD :type Name :default "None"))
  ;[1 1 1] interface setId
  (Variables|Default|Setid ""))

(event EventCloseMenu
  ;[1 1 1] interface closeMenu
  (Actor|DestroyActor))

(event EventSetText
  (params (String :type String) (Option :type Integer))
  (bind _returnvalue (Utilities|Text|ToText(String) String))
  ;[1 1 1] Interface setText
  (switch int Option
    (:Default
      (Rendering|Components|TextRender|SetText (Variables|Default|GetText1) _returnvalue :!label _label))
    (:0
      (goto _label))
    (:1
      (Class|BPIOption|SetText(Message) (Variables|/Script/Engine.ChildActorComponent|GetChildActor (Variables|Default|GetOption1)) _returnvalue))
    (:2
      (Class|BPIOption|SetText(Message) (Variables|/Script/Engine.ChildActorComponent|GetChildActor (Variables|Default|GetOption2)) _returnvalue))))

(fn ConstructionScript)

(fn InitSelf
  (bind _self self)
  (Rendering|Components|TextRender|SetText (Variables|Default|GetText1) (Class|KismetTextLibrary|GetEmptyText))
  (Class|BPIOption|SetMenu(Message) (Variables|/Script/Engine.ChildActorComponent|GetChildActor (Variables|Default|GetOption1)) _self)
  (Class|BPIOption|SetMenu(Message) (Variables|/Script/Engine.ChildActorComponent|GetChildActor (Variables|Default|GetOption2)) _self)
  (return))