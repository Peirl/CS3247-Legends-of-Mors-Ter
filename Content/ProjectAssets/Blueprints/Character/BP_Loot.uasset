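; BP_Loot is a gold pickup actor that rewards a DragonCharacter on overlap with its capsule.
; The overlap adds GoldValue to that character's gold and sets the Message text to the looted amount.
; It then toggles visibility on the GoldBag and Message components and destroys the actor after a short delay.
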(event OnComponentBeginOverlap(Capsule)
  (params (OtherActor :type Actor%20Object%20Reference) (OtherComp :type Primitive%20Component%20Object%20Reference) (OtherBodyIndex :type Integer) (bFromSweep :type Boolean) (SweepResult :type Hit%20Result%20Structure%20%28by%20ref%29))
  (bind _asdragon_character (Utilities|Casting|CastToDragonCharacter OtherActor))
  (Default|IncreaseGold _asdragon_character (Variables|Default|GetGoldValue))
  (Rendering|Components|TextRender|SetText (Variables|Default|GetMessage) (Utilities|Text|ToText(String) (Utilities|String|Append (Utilities|String|ToString(Integer) (Variables|Default|GetGoldValue)) " gold looted")))
  (Rendering|ToggleVisibility (Variables|Default|GetGoldBag) true)
  (Rendering|ToggleVisibility (Variables|Default|GetMessage) false)
  (Utilities|FlowControl|Delay 3.0)
  (Actor|DestroyActor))

(event EventBeginPlay)

(event EventActorBeginOverlap
  (params (OtherActor :type Actor%20Object%20Reference)))

(event EventTick
  (params (DeltaSeconds :type Float%20%28single-precision%29)))

(fn ConstructionScript)