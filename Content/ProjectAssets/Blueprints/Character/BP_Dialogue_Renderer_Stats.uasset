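; Dialogue renderer that shows the player's stats panel, titled "Mors Terriblis", with gold, HP and Human and Fae favour.
; On BeginPlay it takes the first DragonCharacter, caches those values from its getters and writes them into five text components via SetTextSelf.
; It then spawns a Stats_close option at the first option component, linked to this renderer with "End" as the next dialogue.
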(event EventBeginPlay
  (bind _self self)
  (bind _player (Variables|Default|Getplayer))
  (|CallParentFunction)
  (bind _outactors (Actor|GetAllActorsOfClass "/Game/ProjectAssets/Blueprints/Character/DragonCharacter.DragonCharacter_C"))
  (Variables|Default|SetPlayer (Utilities|Array|Get(acopy) _outactors))
  (bind _gold (Class|BPICharacter|GetGold(Message) _player))
  (Variables|Default|SetGold _gold)
  (bind _maxhp (Class|BPICharacter|GetMaxHP(Message) _player))
  (Variables|Default|SetMaxHP _maxhp)
  (bind _hp (Class|BPICharacter|GetHP(Message) _player))
  (Variables|Default|SetHP _hp)
  (bind _fame (Class|BPICharacter|GetHumanFame(Message) _player))
  (Variables|Default|SethumanAlignment _fame)
  (bind _fame_2 (Default|GetFaeFame _player))
  (Variables|Default|SetfaeAlignment _fame_2)
  (CallFunction|SetTextSelf)
  (bind _returnvalue (Game|SpawnActorfromClass "/Game/ProjectAssets/Blueprints/Character/DialogueOptions/stats_close.stats_close_C" (Transformation|GetWorldTransform (Utilities|Array|Get(acopy) (Variables|Default|GetoptionComponents))) "Undefined" _self _self "End"))
  (Utilities|Array|Add (Variables|Default|GetoptionsCreated) _returnvalue))

(fn ConstructionScript
  (|CallParentFunction))

(fn SetTextSelf
  (Rendering|Components|TextRender|SetText (Variables|Default|GetText1) (Utilities|Text|ToText(String) (Utilities|String|MakeLiteralString "Mors Terriblis ")))
  (Rendering|Components|TextRender|SetText (Variables|Default|GetText2) (Utilities|Text|ToText(String) (Utilities|String|Append (Utilities|String|MakeLiteralString "Gold: ") (Utilities|String|ToString(Integer) (Variables|Default|GetGold)))))
  (Rendering|Components|TextRender|SetText (Variables|Default|GetText3) (Utilities|Text|ToText(String) (Utilities|String|Append (Utilities|String|MakeLiteralString "HP: ") (Utilities|String|ToString(Float) (Variables|Default|GetHP)) "/" (Utilities|String|ToString(Float) (Variables|Default|GetMaxHP)))))
  (Rendering|Components|TextRender|SetText (Variables|Default|GetText4) (Utilities|Text|ToText(String) (Utilities|String|Append (Utilities|String|MakeLiteralString "Human Favour: ") (Utilities|String|ToString(Integer) (Variables|Default|GetHumanAlignment)))))
  (Rendering|Components|TextRender|SetText (Variables|Default|GetText5) (Utilities|Text|ToText(String) (Utilities|String|Append (Utilities|String|MakeLiteralString "Fae Favour: ") (Utilities|String|ToString(Integer) (Variables|Default|GetFaeAlignment)))))
  (return))