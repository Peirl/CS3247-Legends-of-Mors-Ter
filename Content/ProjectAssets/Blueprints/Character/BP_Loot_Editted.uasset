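; Gold loot pickup Actor that credits its GoldValue to a DragonCharacter overlapping its Box.
; Tick uses a DoOnce to give high-value loot a treasure mesh, rotating the actor and prompt and repositioning the message.
; On overlap it sets the looted-amount text, toggles bag and message visibility, then destroys itself after a delay.
; Nothing disables the overlap during that delay.
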(event OnComponentBeginOverlap(Box)
  (params (OtherActor :type Actor%20Object%20Reference) (OtherComp :type Primitive%20Component%20Object%20Reference) (OtherBodyIndex :type Integer) (bFromSweep :type Boolean) (SweepResult :type Hit%20Result%20Structure%20%28by%20ref%29))
  (bind _asdragon_character (Utilities|Casting|CastToDragonCharacter OtherActor))
  (Default|IncreaseGold _asdragon_character (Variables|Default|GetGoldValue))
  (Rendering|Components|TextRender|SetText (Variables|Default|GetMessage) (Utilities|Text|ToText(String) (Utilities|String|Append (Utilities|String|ToString(Integer) (Variables|Default|GetGoldValue)) " gold looted")))
  (Rendering|ToggleVisibility (Variables|Default|GetGoldBag) true)
  (Rendering|ToggleVisibility (Variables|Default|GetMessage) false)
  (Utilities|FlowControl|Delay 5.0)
  (Actor|DestroyActor))

(event EventActorBeginOverlap
  (params (OtherActor :type Actor%20Object%20Reference)))

(event EventTick
  (params (DeltaSeconds :type Float%20%28single-precision%29))
  (if (>= (Variables|Default|GetGoldValue) 50)
    (Utilities|FlowControl|DoOnce false
      (:Completed
        (Components|StaticMesh|SetStaticMesh (Variables|Default|GetGoldBag) "/Game/InfinityBladeFireLands/Environments/Fire/Env_Fire_Rocky/StaticMesh/SM_Fire_Treasure002.SM_Fire_Treasure002")
        (Transformation|SetActorRotation "0,270.000000, 0")
        (Transformation|SetWorldRotation (Variables|Default|GetPrompt) "0,270.000000, 0" false false)
        (Transformation|SetWorldLocationAndRotation (Variables|Default|GetMessage) (+ (Transformation|GetActorLocation) "0.000000,500.000000,200.000000") "0,270.000000, 0" false false)))))

(fn ConstructionScript)