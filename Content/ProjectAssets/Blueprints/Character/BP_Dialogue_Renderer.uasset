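; BP_Dialogue_Renderer is an actor that displays branching dialogue in the world, starting from DialogueName on BeginPlay.
; Each Dialogues data table row fills up to six text render components, split by line and tinted by a colour field.
; It spawns the row's option actors at two option components, each carrying its next row name.
; Callback renders the selected option's next row; "End" or CloseMenu clears everything and destroys the actor.
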(event EventCallback
  (params (selectedOption :type BPI%20Option%20Interface))
  (bind _nextdialogue (Default|GetNextDialogue selectedOption))
  (CallFunction|RenderNext _nextdialogue))

(event EventBeginPlay
  (CallFunction|RenderNext (Variables|Default|GetdialogueName)))

(event EventCloseMenu
  ;[1 1 1] interface closeMenu
  (CallFunction|ClearDialogue)
  (Actor|DestroyActor))

(fn ConstructionScript
  (Utilities|Array|Insert (Variables|Default|GettextComponents) (Variables|Default|GetText1))
  (Utilities|Array|Insert (Variables|Default|GettextComponents) (Variables|Default|GetText2) 1)
  (Utilities|Array|Insert (Variables|Default|GettextComponents) (Variables|Default|GetText3) 2)
  (Utilities|Array|Insert (Variables|Default|GettextComponents) (Variables|Default|GetText4) 3)
  (Utilities|Array|Insert (Variables|Default|GettextComponents) (Variables|Default|GetText5) 4)
  (Utilities|Array|Insert (Variables|Default|GettextComponents) (Variables|Default|GetText6) 5)
  (Utilities|Array|Insert (Variables|Default|GetoptionComponents) (Variables|Default|GetOption1))
  (Utilities|Array|Insert (Variables|Default|GetoptionComponents) (Variables|Default|GetOption2) 1))

(fn Render
  (params (dialogue :type Dialogue%20Struct%20Structure))
  (bind (_text _colour _option_text _nextdiaglogues _context _options) (Utilities|Struct|BreakDialogue_struct dialogue))
  (bind _self self)
  (Utilities|FlowControl|Sequence
    (:then_0
      (for (_array_element _array_index) (Utilities|String|ParseIntoArray _text "\\n")
        (Rendering|Components|TextRender|SetText (Utilities|Array|Get(acopy) (Variables|Default|GettextComponents) _array_index) (Utilities|Text|ToText(String) _array_element))
        (switch int _colour
          (:Default
            (Rendering|Components|TextRender|SetTextRenderColor (Utilities|Array|Get(acopy) (Variables|Default|GettextComponents) _array_index) (Math|Color|MakeColor 0 0 0) :!label _label))
          (:0
            (goto _label))
          (:1
            (Rendering|Components|TextRender|SetTextRenderColor (Utilities|Array|Get(acopy) (Variables|Default|GettextComponents) _array_index) (Math|Color|MakeColor 0 0 100)))
          (:2
            (Rendering|Components|TextRender|SetTextRenderColor (Utilities|Array|Get(acopy) (Variables|Default|GettextComponents) _array_index) (Math|Color|MakeColor 0 100 0)))
          (:3
            (Rendering|Components|TextRender|SetTextRenderColor (Utilities|Array|Get(acopy) (Variables|Default|GettextComponents) _array_index) (Math|Color|MakeColor 100 0 0))))))
    (:then_1
      (for (_array_element_2 _array_index_2) _options
        (bind _returnvalue (Game|SpawnActorfromClass _array_element_2 (Transformation|GetWorldTransform (Utilities|Array|Get(acopy) (Variables|Default|GetoptionComponents) _array_index_2)) "Undefined" _self _self (Utilities|Array|Get(acopy) _nextdiaglogues _array_index_2)))
        (Utilities|Array|Add (Variables|Default|GetoptionsCreated) _returnvalue)))))

(fn ClearDialogue
  (Utilities|FlowControl|Sequence
    (:then_0
      (for _array_element (Variables|Default|GettextComponents)
        (if (Utilities|IsValid _array_element)
          (Rendering|Components|TextRender|SetText _array_element (Utilities|Text|ToText(String) (Utilities|String|MakeLiteralString))))))
    (:then_1
      (for _array_element_2 (Variables|Default|GetoptionsCreated)
        (if (Utilities|IsValid _array_element_2)
          (Actor|DestroyActor _array_element_2))))
    (:then_2
      (Utilities|Array|Clear (Variables|Default|GetoptionsCreated)))))

(fn RenderNext
  (params (dialogue :type Name))
  (if (Utilities|Name|NotEqual(Name) dialogue "End")
    (bind _returnvalue (Utilities|GetDataTableRow "/Game/ProjectAssets/Blueprints/Character/Dialogues.Dialogues" dialogue)
      (:then
        (CallFunction|ClearDialogue)
        (CallFunction|Render _returnvalue)))
    (else
      (CallFunction|CloseMenu))))