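; BP_Menu_OptionA is a menu option with a text render label, driven through interface events.
; Hover on and hover off change the label's colour, and SetText replaces its text.
; SetSelect stores a selection string, which Select only prints, with no further menu action.
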(event EventSetSelect
  (params (String :type String))
  ;[1 1 1] Set Selection
  (Variables|Default|Setselection String))

(event EventSetText
  (params (Test :type Text))
  ;[1 1 1] Interface setText
  (Rendering|Components|TextRender|SetText (Variables|Default|GetText) Test))

(event EventSelect
  ;[1 1 1] Interface select
  (Development|PrintString (Variables|Default|Getselection)))

(event EventHoveron
  ;[1 1 1] Interface Hover on
  (Rendering|Components|TextRender|SetTextRenderColor (Variables|Default|GetText) (Math|Color|MakeColor 1 1 1)))

(event EventHoverOff
  ;[1 1 1] Interface HoverOff
  (Rendering|Components|TextRender|SetTextRenderColor (Variables|Default|GetText) (Math|Color|MakeColor 0 0 0)))

(fn ConstructionScript)