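; BP_Option is a selectable dialogue option shown as in-world text through a TextRender component.
; Interface events switch the text to white on hover, restore a default color on hover-off, and update the displayed string.
; Selection runs DoAction, then passes the option itself to its Renderer through CallbackMessage.
; The construction script applies the Text variable, and GetNextDialogue exposes the dialogue that follows this option.
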(event EventSelect
  ;[1 1 1] Interface select
  (CallFunction|DoAction)
  (Class|BPIMenu|Callback(Message) (Variables|Default|Getrenderer) self))

(event EventSetText
  (params (Test :type Text))
  ;[1 1 1] Interface setText
  (Rendering|Components|TextRender|SetText (Variables|Default|GetTextRender) Test))

(event EventHoveron
  ;[1 1 1] Interface Hover on
  (Rendering|Components|TextRender|SetTextRenderColor (Variables|Default|GetTextRender) (Math|Color|MakeColor 255 255 255)))

(event EventHoverOff
  ;[1 1 1] Interface HoverOff
  (Rendering|Components|TextRender|SetTextRenderColor (Variables|Default|GetTextRender) (Math|Color|MakeColor 0 0 0)))

(fn ConstructionScript
  (Rendering|Components|TextRender|SetText (Variables|Default|GetTextRender) (Variables|Default|Gettext)))

(fn GetNextDialogue
  (return (Variables|Default|GetnextDialogue)))